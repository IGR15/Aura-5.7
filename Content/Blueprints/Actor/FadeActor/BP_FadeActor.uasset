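; BP_FadeActor is an actor whose static mesh fades out and back in through a timeline-driven "Fade" material parameter.
; Construction caches original materials and builds dynamic instances from FadeMaterialInstances.
; FadeOut swaps these in and plays the timeline; FadeIn reverses it.
; On finish, a value of 0 makes a custom trace channel, and optionally Visibility, ignore the mesh, while 1 restores original materials and blocking.
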(event `/Game/Blueprints/Actor/FadeActor/BI_FadeInterface.FadeOut`
  (`self.setMaterial To Dynamic Instancses`)
  (bind (_direction _fade) (`Timeline|FadeTimeline` :!label _label)
    (:`Update`
      (for _array_element (`self.DynamicMaterialInstances`)
        (`MaterialInstanceDynamic.SetScalarParameterValue` _array_element "Fade" _fade)))
    (:`Finished`
      (`self.FadeOutEnd` _fade))))

(event `/Game/Blueprints/Actor/FadeActor/BI_FadeInterface.FadeIn`
  (goto _label :!via `Reverse`))

(event `self.ReceiveBeginPlay`)

(fn `FadeOutEnd`
  (params (InputPin :type "Float (single-precision)"))
  (if (>= InputPin 1.0)
    (`self.Reset Material Instances`)
    (`PrimitiveComponent.SetCollisionResponseToChannel` (`self.StaticMesh`) "ECC_GameTraceChannel2" "ECR_Block")
    (if (`self.BlockVisibility`)
      (`PrimitiveComponent.SetCollisionResponseToChannel` (`self.StaticMesh`) "ECC_Visibility" "ECR_Block"))
    (elif (<= InputPin 0.0)
      (`PrimitiveComponent.SetCollisionResponseToChannel` (`self.StaticMesh`) "ECC_GameTraceChannel2" "ECR_Ignore")
      (if (`self.BlockVisibility`)
        (`PrimitiveComponent.SetCollisionResponseToChannel` (`self.StaticMesh`) "ECC_Visibility" "ECR_Ignore")))))

(fn `Reset Material Instances`
  (for (_array_element _array_index) (`self.OriginalMaterial`)
    (`PrimitiveComponent.SetMaterial` (`self.StaticMesh`) _array_index _array_element)))

(fn `setMaterial To Dynamic Instancses`
  (for (_array_element _array_index) (`self.DynamicMaterialInstances`)
    (`PrimitiveComponent.SetMaterial` (`self.StaticMesh`) _array_index _array_element)))

(fn `UserConstructionScript`
  (`KismetArrayLibrary.Array_Clear` (`self.DynamicMaterialInstances`))
  (set `self.OriginalMaterial` (`MeshComponent.GetMaterials` (`self.StaticMesh`)))
  (for _array_element (`self.FadeMaterialInstances`)
    (bind _returnvalue (`KismetMaterialLibrary.CreateDynamicMaterialInstance` _array_element))
    (`KismetArrayLibrary.Array_AddUnique` (`self.DynamicMaterialInstances`) _returnvalue)))