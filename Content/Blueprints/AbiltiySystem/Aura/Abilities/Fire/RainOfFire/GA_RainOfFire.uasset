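; Gameplay ability for Aura's Rain of Fire spell, which drops a staggered series of fire projectiles around a targeted point.
; Activation shows a magic circle on the avatar, waits for an input press, then takes the impact point under the mouse.
; It generates random points raised above that area, and a looping timer calls SpawnNextFireRain at each one.
; Once every point is used, the timer clears and the ability ends.
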(event `self.K2_ActivateAbility`
  (`|ExecutionSequence`
    (:`then_0`
      (message `PlayerInterface.ShowMagicCircle` (`self.GetAvatarActorFromActorInfo`) null))
    (:`then_1`
      (`AbilityTask_WaitInputPress.WaitInputPress` false
        (:`OnPress`
          (bind (_asynctaskproxy _datahandle) (`TargetDataUnderMouse.CreateTargetDataUnderMouse`)
            (:`ValidData`
              (set `self.Impact Point` (`.ImpactPoint` (`GameplayStatics.BreakHitResult` (`AbilitySystemBlueprintLibrary.GetHitResultFromTargetData` _datahandle))))
              (`|ExecutionSequence`
                (:`then_0`
                  (bind _returnvalue (`self.GetRandomPointsInRadius` (`self.Impact Point`) 400.0 (`self.Num Points`) 400.0))
                  (set `self.RandomPoint` _returnvalue))
                (:`then_1`
                  (bind _returnvalue_2 (`KismetSystemLibrary.K2_SetTimerDelegate` (delegate `SpawnFIreball`) (`self.Spawn timer delta time`) true))
                  (set `self.FireBallSpwan Timer` _returnvalue_2)
                  (`self.SpawnFIreball`))))))))))

(event `SpawnFIreball`
  (if (< (`self.Count`) (`self.Num Points`))
    (set `self.SpawnLocation` (`|GetArrayItem` (`self.RandomPoint`) (`self.Count`)))
    (`/Engine/EditorBlueprintResources/StandardMacros.IncrementInt` (`self.Count`)
      (:`  `
        (`self.SpawnNextFireRain` (`self.SpawnLocation`))))
    (else
      (`KismetSystemLibrary.K2_ClearAndInvalidateTimerHandle` (`self.FireBallSpwan Timer`))
      (`self.K2_EndAbility`))))